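; AutoMortar2 is a mortar Blueprint built on tank components, with a barrel, a turret, an aiming component and a health bar widget.
; On BeginPlay it initialises TankAiming with its barrel and turret.
; It then sets itself as OwningTank on the HealthBar widget.
; The graphs contain only this setup, with no firing or targeting logic.
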(event `self.ReceiveBeginPlay`
  (`TankAimingComponent.Initialise` (`self.TankAiming`) (`self.TankBarrel`) (`self.TankTurret`))
  (`self.InitializeHealthBar`))

(fn `InitializeHealthBar`
  (set `/Game/Blueprints/UI/HealthBar.OwningTank` self (cast `/Game/Blueprints/UI/HealthBar` (`WidgetComponent.GetUserWidgetObject` (`self.HealthBar`)) :!pure true))
  (return))

(fn `UserConstructionScript`)