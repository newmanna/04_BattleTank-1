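; Player-controlled tank pawn that binds input to driving, aiming and firing.
; BeginPlay hands tracks to TankMovement, barrel and turret to TankAiming, and links the health bar widget to the tank.
; Axes drive movement intents and rotate the azimuth gimbal and spring arm; Swap Cam toggles both cameras on press and release, giving a hold-to-switch view.
; Unconnected leftovers include a socket-trace track suspension force and a radial damage call.
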(event `self.ReceiveBeginPlay`
  (`TankMovementComponent.Initialise` (`self.TankMovement`) (`self.TankTrack_Left`) (`self.TankTrack_Right`))
  (`TankAimingComponent.Initialise` (`self.TankAiming`) (`self.TankBarrel`) (`self.TankTurret`))
  (`self.Initialize HealthBarWidget`))

(event `InputAxis|Aim Elevation `
  (params (AxisValue :type "Float (single-precision)"))
  ;[1 1 1] InputBinding
  (`SceneComponent.K2_AddLocalRotation` (`self.SpringArm`) (`KismetMathLibrary.MakeRotator` 0.0 (* AxisValue (`GameplayStatics.GetWorldDeltaSeconds`) 100.0)) false false))

(event `self.ReceiveTick`
  (params (DeltaSeconds :type "Float (single-precision)")))

(event `InputAxis|Aim Azimuth`
  (params (AxisValue :type "Float (single-precision)"))
  ;[1 1 1] InputBinding
  (`SceneComponent.K2_AddLocalRotation` (`self.AzimuthGimbal`) (`KismetMathLibrary.MakeRotator` 0.0 0.0 (* AxisValue (`GameplayStatics.GetWorldDeltaSeconds`) 100.0)) false false))

(event `InputAction|Fire`
  (params (Key :type "Key Structure" :default "AnyKey"))
  ;[1 1 1] InputBinding
  (:`Pressed`
    (`TankAimingComponent.Fire` (`self.TankAiming`))))

(event `InputAxis|MoveForward`
  (params (AxisValue :type "Float (single-precision)"))
  (`TankMovementComponent.IntendMoveForward` (`self.TankMovement`) AxisValue))

(event `InputAction|Swap Cam`
  (params (Key :type "Key Structure" :default "AnyKey"))
  (:`Pressed`
    (`ActorComponent.ToggleActive` (`self.CameraThirtPerson`) :!label _label)
    (`ActorComponent.ToggleActive` (`self.CameraFirstPerson`)))
  (:`Released`
    (goto _label)))

(event `InputAxis|TurnRight`
  (params (AxisValue :type "Float (single-precision)"))
  (`TankMovementComponent.IntendTurnRight` (`self.TankMovement`) AxisValue))

(event `Key|LeftShift`
  (params (Key :type "Key Structure" :default "AnyKey")))

(fn `Initialize HealthBarWidget`
  (set `/Game/Blueprints/UI/HealthBar.OwningTank` self (cast `/Game/Blueprints/UI/HealthBar` (`WidgetComponent.GetUserWidgetObject` (`self.HealthBar`)) :!pure true))
  (return))

(fn `UserConstructionScript`)