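; Procedural terrain actor built around a RuntimeMeshComponent, whose only active logic is a runtime navmesh workaround.
; After a delay on BeginPlay, it nudges itself up and back down to trigger navmesh generation, which the author marks as a temporary hack.
; Tick and the construction script are empty.
; Mesh generation with timing, landscape material assignment, per-section debug markers and player-position debug drawing remain as disconnected, never-executed nodes.
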(event `self.ReceiveBeginPlay`
  ;[1 1 1] temporal hack to get navmesh to generate in runtime
  (`KismetSystemLibrary.Delay` 5.0)
  (`self.K2_SetActorLocation` (+ (`self.K2_GetActorLocation`) (0.0 0.0 1.0)))
  (`self.K2_SetActorLocation` (+ (`self.K2_GetActorLocation`) (0.0 0.0 -1.0))))

(event `self.ReceiveTick`
  (params (DeltaSeconds :type "Float (single-precision)")))

(fn `UserConstructionScript`
  (locals (ConstructBeginTime :type "DateTime Structure")))