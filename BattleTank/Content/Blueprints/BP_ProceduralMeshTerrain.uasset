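; Procedural mesh terrain actor that builds its mesh at construction time.
; The construction script calls GenerateMesh, whose body is not in this file, then logs the elapsed build time in seconds and milliseconds without showing it on screen.
; The only active event, AnyDamage, prints the damage amount received.
; BeginPlay, overlap and Tick are disabled stubs, and some leftover clear and loop nodes never run.
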(event EventBeginPlay)

(event Collision|EventActorBeginOverlap
  (params (OtherActor :type Actor%20Object%20Reference)))

(event EventTick
  (params (DeltaSeconds :type Float%20%28single-precision%29)))

(event Game|Damage|EventAnyDamage
  (params (Damage :type Float%20%28single-precision%29) (DamageType :type Damage%20Type%20Object%20Reference) (InstigatedBy :type Controller%20Object%20Reference) (DamageCauser :type Actor%20Object%20Reference))
  (Development|PrintString (Utilities|String|ToString(Float) Damage)))

(fn ConstructionScript
  (LocalVariables|SetConstructionTime (Math|DateTime|UTCNow))
  (Class|ProceduralMeshTerrain|GenerateMesh true)
  (Development|PrintString (Utilities|String|Append "Construction: " (Utilities|String|ToString(Integer) (.second (- (Math|DateTime|UTCNow) (Math|Timespan|MakeTimespan (.day (LocalVariables|GetConstructionTime)) (.hour (LocalVariables|GetConstructionTime)) (.minute (LocalVariables|GetConstructionTime)) (.second (LocalVariables|GetConstructionTime)) (.millisecond (LocalVariables|GetConstructionTime)))))) "s " (Utilities|String|ToString(Integer) (.millisecond (- (Math|DateTime|UTCNow) (Math|Timespan|MakeTimespan (.day (LocalVariables|GetConstructionTime)) (.hour (LocalVariables|GetConstructionTime)) (.minute (LocalVariables|GetConstructionTime)) (.second (LocalVariables|GetConstructionTime)) (.millisecond (LocalVariables|GetConstructionTime)))))) "ms") false true "(R=1.000000,G=0.941491,B=0.911000,A=1.000000)"))