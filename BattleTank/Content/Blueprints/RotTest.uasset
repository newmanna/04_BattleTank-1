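; RotTest is a test actor that approximates arm IK with Shoulder, Elbow and Hand components in the Construction Script.
; Hand follows IKHand along the shoulder direction, clamped to MaxLength.
; Elbow sits at the Shoulder-Hand midpoint, pushed perpendicular by half the unused reach via a look-at rotation pitched 90 degrees, a linear bend without trigonometric solving.
; Event graph is empty; leftover shoulder rotation and elbow offset nodes are disconnected.
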(fn `GetDistance`
  (params (from :type "StaticMeshComponent Object Reference") (to :type "StaticMeshComponent Object Reference"))
  (returns (length :type "Float (double-precision)"))
  (return (`KismetMathLibrary.VSize` (- (`SceneComponent.K2_GetComponentLocation` from) (`SceneComponent.K2_GetComponentLocation` to)))))

(fn `GetPositionInbetween`
  (params (`1` :type "StaticMeshComponent Object Reference") (`2` :type "StaticMeshComponent Object Reference"))
  (returns (middle :type "Vector Structure"))
  (return (`KismetMathLibrary.GetVectorArrayAverage` (`|MakeArray` (`SceneComponent.K2_GetComponentLocation` `1`) (`SceneComponent.K2_GetComponentLocation` `2`)))))

(fn `UserConstructionScript`
  (bind _maxlength (`self.MaxLength`))
  (bind _length (`self.GetDistance` (`self.Shoulder`) (`self.IK Hand`)))
  (bind (_returnvalue_roll _returnvalue_pitch _returnvalue_yaw) (`KismetMathLibrary.BreakRotator` (`KismetMathLibrary.FindLookAtRotation` (`SceneComponent.K2_GetComponentLocation` (`self.Shoulder`)) (`SceneComponent.K2_GetComponentLocation` (`self.Hand`)))))
  (bind _returnvalue (select `bool` (> _length _maxlength) :`false` _length :`true` _maxlength))
  (`SceneComponent.K2_SetWorldLocation` (`self.Hand`) (+ (`SceneComponent.K2_GetComponentLocation` (`self.Shoulder`)) (* (`KismetMathLibrary.GetDirectionVector` (`SceneComponent.K2_GetComponentLocation` (`self.Shoulder`)) (`SceneComponent.K2_GetComponentLocation` (`self.IK Hand`))) _returnvalue)) false false)
  (`SceneComponent.K2_SetWorldLocation` (`self.Elbow`) (+ (`self.GetPositionInbetween` (`self.Shoulder`) (`self.Hand`)) (`KismetMathLibrary.GreaterGreater_VectorRotator` (`KismetMathLibrary.MakeVector` (/ (- _returnvalue (`self.MaxLength`)) 2.0)) (`KismetMathLibrary.MakeRotator` _returnvalue_roll (- _returnvalue_pitch -90.0) _returnvalue_yaw))) false false))