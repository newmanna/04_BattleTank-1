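; Player-controlled tank pawn that passes drive, turn and fire input to TankMovement and TankAiming, with aim axes rotating the camera gimbal and spring arm.
; Each tick, hover-style suspension line-traces along the forward axis of every track socket.
; Hits within range push the body at that socket along the same axis, fading linearly with distance.
; Force is split across each track's sockets, divided by delta time and halved while the track moves.
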(event `self.ReceiveBeginPlay`
  (`TankMovementComponent.Initialise` (`self.TankMovement`) (`self.TankTrack_Left`) (`self.TankTrack_Right`))
  (`TankAimingComponent.Initialise` (`self.TankAiming`) (`self.TankBarrel`) (`self.TankTurret`)))

(event `InputAxis|Aim Elevation `
  (params (AxisValue :type "Float (single-precision)"))
  ;[1 1 1] InputBinding
  (`SceneComponent.K2_AddLocalRotation` (`self.SpringArm`) (`KismetMathLibrary.MakeRotator` 0.0 (* AxisValue (`GameplayStatics.GetWorldDeltaSeconds`) 100.0)) false false))

(event `self.ReceiveTick`
  (params (DeltaSeconds :type "Float (single-precision)"))
  (bind _desiredtracelength (`self.DesiredTraceLength`))
  (for _array_element (`|MakeArray` (`self.TankTrack_Left`) (`self.TankTrack_Right`))
    (bind _returnvalue (`SceneComponent.GetAllSocketNames` _array_element))
    (for _array_element_2 _returnvalue
      (bind (_returnvalue_location _returnvalue_rotation) (`KismetMathLibrary.BreakTransform` (`SceneComponent.GetSocketTransform` _array_element _array_element_2 "RTS_World")))
      (bind _outhit (`KismetSystemLibrary.LineTraceSingle` :`Start` _returnvalue_location :`End` (+ _returnvalue_location (* (`KismetMathLibrary.GetForwardVector` _returnvalue_rotation) (`self.DesiredTraceLength`))) :`TraceChannel` "TraceTypeQuery1" :`DrawDebugType` "ForOneFrame"))
      (bind (_bblockinghit _binitialoverlap _time _location _impactpoint _normal _impactnormal _physmat _hitactor _hitcomponent _hitbonename _hititem _tracestart) (`GameplayStatics.BreakHitResult` _outhit))
      (bind _returnvalue_2 (`KismetMathLibrary.VSize` (- _location _tracestart)))
      (if (< _returnvalue_2 _desiredtracelength)
        (`PrimitiveComponent.AddForceAtLocation` (`self.TankBody`) (* (`KismetMathLibrary.GetForwardVector` _returnvalue_rotation) (`KismetMathLibrary.Lerp` (* (/ (/ (`self.DesiredForcePerTrack`) (`KismetMathLibrary.Conv_IntToDouble` (`KismetArrayLibrary.Array_Length` _returnvalue))) (`GameplayStatics.GetWorldDeltaSeconds`)) (select `bool` (> (`KismetMathLibrary.VSize` (`SceneComponent.GetComponentVelocity` _array_element)) 0.0) :`false` 1.0 :`true` 0.5 :!type "Float (single-precision)")) 0.0 (/ _returnvalue_2 _desiredtracelength))) _tracestart "None")))))

(event `InputAxis|Aim Azimuth`
  (params (AxisValue :type "Float (single-precision)"))
  ;[1 1 1] InputBinding
  (`SceneComponent.K2_AddLocalRotation` (`self.AzimuthGimbal`) (`KismetMathLibrary.MakeRotator` 0.0 0.0 (* AxisValue (`GameplayStatics.GetWorldDeltaSeconds`) 100.0)) false false))

(event `InputAction|Fire`
  (params (Key :type "Key Structure" :default "AnyKey"))
  ;[1 1 1] InputBinding
  (:`Pressed`
    (`TankAimingComponent.Fire` (`self.TankAiming`))))

(event `InputAxis|MoveForward`
  (params (AxisValue :type "Float (single-precision)"))
  (`TankMovementComponent.IntendMoveForward` (`self.TankMovement`) AxisValue))

(event `InputAxis|TurnRight`
  (params (AxisValue :type "Float (single-precision)"))
  (`TankMovementComponent.IntendTurnRight` (`self.TankMovement`) AxisValue))

(event `Key|LeftShift`
  (params (Key :type "Key Structure" :default "AnyKey")))

(fn `UserConstructionScript`)